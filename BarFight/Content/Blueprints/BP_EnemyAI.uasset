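; BP_EnemyAI is an enemy pawn that chases the player and ragdolls or tumbles when struck by fast-moving objects.
; PawnSensing sets a seen flag, which is never cleared here, and issues an AI MoveTo toward the player character on each sighting.
; Hits from non-player actors above a speed threshold enable mesh physics, deactivate the capsule and apply an impulse scaled from the other actor's velocity at the hit point.
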(event OnSeePawn(PawnSensing)
  (params (Pawn :type Pawn%20Object%20Reference))
  (Variables|Default|SetisSeeingPlayer? true)
  (CallFunction|FollowPlayer))

(event Custom|FollowPlayer
  (if (Variables|Default|GetisSeeingPlayer?)
    (AI|AIMoveTo self "0, 0, 0" (Game|GetPlayerCharacter 0) 5.0 false)))

(event EventBeginPlay)

(event Collision|EventActorBeginOverlap
  (params (OtherActor :type Actor%20Object%20Reference)))

(event EventTick
  (params (DeltaSeconds :type Float%20%28single-precision%29)))

(event Collision|EventHit
  (params (MyComp :type Primitive%20Component%20Object%20Reference) (Other :type Actor%20Object%20Reference) (OtherComp :type Primitive%20Component%20Object%20Reference) (bSelfMoved :type Boolean) (HitLocation :type Vector :default "0, 0, 0") (HitNormal :type Vector :default "0, 0, 0") (NormalImpulse :type Vector :default "0, 0, 0") (Hit :type Hit%20Result%20Structure%20%28by%20ref%29))
  (bind _returnvalue (Transformation|GetVelocity Other))
  (Utilities|Casting|CastToBP_FirstPersonCharacter Other
    (:CastFailed
      (if (> (Math|Vector|VectorLength _returnvalue) 3e+02)
        (Physics|SetSimulatePhysics (Variables|Character|GetMesh) true)
        (Components|Activation|Deactivate (Variables|Collision|GetCapsuleComponent))
        (Physics|AddImpulseatLocation (Variables|Character|GetMesh) (* _returnvalue 1e+02) HitLocation "None")))))

(fn ConstructionScript)