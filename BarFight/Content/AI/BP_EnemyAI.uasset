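; Enemy AI character that chases the player once seen and can be knocked down by fast-moving objects.
; PawnSensing sightings trigger an AI MoveTo toward the player character while the enemy is not down.
; Hits from non-player actors above a speed threshold switch the mesh to ragdoll, apply a velocity-based impulse and play a pitch-randomized smack sound.
; After a delay it reattaches the mesh, plays a get-up montage, then re-enables sensing.
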(event OnSeePawn(PawnSensing)
  (params (Pawn :type Pawn%20Object%20Reference))
  ;[1 1 1] sensing
  (if (not (Variables|Default|GetisDown?))
    (Variables|Default|SetisSeeingPlayer? true)
    (CallFunction|FollowPlayer)))

(event Custom|FollowPlayer
  ;[1 1 1] follow player
  (if (Variables|Default|GetisSeeingPlayer?)
    (AI|AIMoveTo self "0, 0, 0" (Game|GetPlayerCharacter 0) 5.0 false)))

(event Custom|StandUp
  (bind _mesh (Variables|Character|GetMesh))
  ;[1 1 1] stand up
  (if (Variables|Default|GetisDown?)
    (Physics|SetSimulatePhysics (Variables|Character|GetMesh) false)
    (Collision|SetCollisionEnabled (Variables|Collision|GetCapsuleComponent) "QueryAndPhysics")
    (Transformation|AttachComponentToComponent _mesh (Variables|Collision|GetCapsuleComponent) "None" "KeepRelative" "KeepRelative" "KeepRelative" true)
    (Transformation|SetRelativeLocationAndRotation _mesh "0.000000,0.000000,-90.000000" "0.000000,-90.000000,0.000000" false false)
    (Animation|PlayAnimMontage "/Game/DrunkAnims/Getting_Up_Anim_Montage.Getting_Up_Anim_Montage" 1.0 "None")
    (Variables|Default|SetisSeeingPlayer? false)
    (Utilities|FlowControl|Delay 6.0)
    (Variables|Default|SetisDown? false)))

(event EventBeginPlay)

(event Collision|EventActorBeginOverlap
  (params (OtherActor :type Actor%20Object%20Reference)))

(event EventTick
  (params (DeltaSeconds :type Float%20%28single-precision%29)))

(event Collision|EventHit
  (params (MyComp :type Primitive%20Component%20Object%20Reference) (Other :type Actor%20Object%20Reference) (OtherComp :type Primitive%20Component%20Object%20Reference) (bSelfMoved :type Boolean) (HitLocation :type Vector :default "0, 0, 0") (HitNormal :type Vector :default "0, 0, 0") (NormalImpulse :type Vector :default "0, 0, 0") (Hit :type Hit%20Result%20Structure%20%28by%20ref%29))
  (bind _returnvalue (Transformation|GetVelocity Other))
  ;[1 1 1] when hit
  (Utilities|Casting|CastToBP_FirstPersonCharacter Other
    (:CastFailed
      (if (> (Math|Vector|VectorLength _returnvalue) 2.8e+02)
        (Physics|SetSimulatePhysics (Variables|Character|GetMesh) true)
        (Collision|SetCollisionEnabled (Variables|Collision|GetCapsuleComponent) "NoCollision")
        (Physics|AddImpulseatLocation (Variables|Character|GetMesh) (* _returnvalue 25.0) HitLocation "None")
        (bind _returnvalue_2 (Audio|CreateSound2D "/Game/Audio/Table-Smack-1_Cue.Table-Smack-1_Cue" 1.0 1.0 0.0 0))
        (Audio|Parameter|SetFloatParameter _returnvalue_2 "HitPitch" (Math|Random|RandomFloatinRange 0.5 1.3) :!class /Script/AudioExtensions.AudioParameterControllerInterface)
        (Audio|Components|Audio|Play _returnvalue_2 0.0)
        (Variables|Default|SetisDown? true)
        (Utilities|FlowControl|Delay 8.0)
        (CallFunction|StandUp)))))

(fn ConstructionScript)